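; Instrument container that spawns an instrument actor and lets it be dragged around the level with the mouse cursor.
; SpawnInstrument creates an InstrumentClass actor at the cursor's Camera-channel hit point, raised by a fixed height offset.
; While spawning is active, Tick repeats the cursor trace to move that actor along with it.
; SpawnInstrumentStop ends the drag and calls ReleaseItem on the first UI_Main widget it finds.
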(event `SpawnInstrument`
  ;[1 1 1] Spawn Object
  (set `self.isSpawning` true)
  (bind _returnvalue (`|SpawnActorFromClass` "/Game/Blueprints/InstrumentClass.InstrumentClass_C" (`KismetMathLibrary.Conv_VectorToTransform` (+ (`.Location` (`GameplayStatics.BreakHitResult` (`PlayerController.GetHitResultUnderCursorByChannel` (`GameplayStatics.GetPlayerController` 0) "TraceTypeQuery2" false))) (0.0 0.0 600.0))) "Undefined" "OverrideRootScale" null null)))

(event `self.ReceiveTick`
  (params (DeltaSeconds :type "Float (single-precision)"))
  ;[1 1 1] Dragging Object
  (if (`self.isSpawning`)
    (`self.K2_SetActorLocation` (stale `SpawnInstrument` _returnvalue) (+ (`.Location` (`GameplayStatics.BreakHitResult` (`PlayerController.GetHitResultUnderCursorByChannel` (`GameplayStatics.GetPlayerController` 0) "TraceTypeQuery2" false))) (0.0 0.0 600.0)) false false)))

(event `SpawnInstrumentStop`
  (set `self.isSpawning` false)
  (bind _foundwidgets (`WidgetBlueprintLibrary.GetAllWidgetsOfClass` "/Game/Blueprints/UI_Main.UI_Main_C"))
  (`/Game/Blueprints/UI_Main.ReleaseItem` (`|GetArrayItem` _foundwidgets)))

(fn `UserConstructionScript`)