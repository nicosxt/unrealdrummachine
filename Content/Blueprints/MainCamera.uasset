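; MainCamera is a mouse-controlled camera actor that pans with left-drag and rotates with right-drag while manipulation is allowed.
; Pressing left stores an offset from a scaled cursor trace hit, and mouse axis events move the root by that offset plus the current scaled hit.
; The same events apply scaled, inverted axis input as local yaw and pitch on separate pivots, keeping the two rotations independent.
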(event `Move Camera`
  ;[1 1 1] Move Camera
  (if (`self.isDragging`)
    (`SceneComponent.K2_SetWorldLocation` (`self.ROOT`) (+ (`self.dragOffset`) (* (`.Location` (`GameplayStatics.BreakHitResult` (`PlayerController.GetHitResultUnderCursorByChannel` (`GameplayStatics.GetPlayerController` 0) "TraceTypeQuery3" true))) (`self.MoveMultiplier`))) false false)))

(event `LMB Pressed`
  ;[1 1 1] Set isDragging & isRotating & is(left)MousePressed
  (if (`self.allowManipulate`)
    (set `self.isDragging` true)
    ;[1 1 1] Set Move Offset
    (set `self.dragOffset` (- (`SceneComponent.K2_GetComponentLocation` (`self.ROOT`)) (* (`.Location` (`GameplayStatics.BreakHitResult` (`PlayerController.GetHitResultUnderCursorByChannel` (`GameplayStatics.GetPlayerController` 0) "TraceTypeQuery3" true))) (`self.MoveMultiplier`))))))

(event `LMB Released`
  ;[1 1 1] Set isDragging & isRotating & is(left)MousePressed
  (set `self.isDragging` false))

(event `RMB Pressed`
  ;[1 1 1] Set isDragging & isRotating & is(left)MousePressed
  (if (`self.allowManipulate`)
    (set `self.isRotating` true)))

(event `RMB Released`
  ;[1 1 1] Set isDragging & isRotating & is(left)MousePressed
  (set `self.isRotating` false))

(event `InputAxisKey|MouseX`
  (params (AxisValue :type "Float (single-precision)"))
  (`self.Move Camera` :!label _label)
  (`self.Rotate Camera X`)
  (`self.Rotate Camera Y`))

(event `InputAxisKey|MouseY`
  (params (AxisValue :type "Float (single-precision)"))
  (goto _label))

(event `Rotate Camera X`
  ;[1 1 1] Rotate Camera
  (if (`self.isRotating`)
    (`SceneComponent.K2_AddLocalRotation` (`self.XPivot`) (`KismetMathLibrary.MakeRotator` 0.0 0.0 (* (stale `InputAxisKey|MouseX` AxisValue) (`self.RotateMultiplier`) -1.0)) false false)))

(event `Rotate Camera Y`
  ;[1 1 1] Rotate Camera
  (if (`self.isRotating`)
    (`SceneComponent.K2_AddLocalRotation` (`self.YPivot`) (`KismetMathLibrary.MakeRotator` 0.0 (* (stale `InputAxisKey|MouseY` AxisValue) (`self.RotateMultiplier`) -1.0)) false false)))

(fn `UserConstructionScript`)