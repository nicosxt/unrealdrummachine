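; Player controller for a puzzle game that creates the main UI widget on start and forwards mouse input to the camera.
; Left and right mouse presses and releases set state flags and call matching handlers on the MainCamera actor found in the level.
; A DragActor event moves a given actor to the hit point of a trace from the camera through a screen position.
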(event `self.ReceiveBeginPlay`
  ;[1 1 1] Create UI On Start
  (bind _returnvalue (`|CreateWidget` "/Game/Blueprints/UI_Main.UI_Main_C"))
  (`UserWidget.AddToViewport` _returnvalue 0))

(event `Key|LeftMouseButton`
  (params (Key :type "Key Structure"))
  (:`Pressed`
    (set `self.leftMousePressed` true)
    ;[1 1 1] Camera Controls
    (bind _returnvalue (`GameplayStatics.GetActorOfClass` "/Game/Blueprints/MainCamera.MainCamera_C"))
    (`/Game/Blueprints/MainCamera.LMB Pressed` _returnvalue))
  (:`Released`
    (set `self.leftMousePressed` false)
    (bind _returnvalue_2 (`GameplayStatics.GetActorOfClass` "/Game/Blueprints/MainCamera.MainCamera_C"))
    (`/Game/Blueprints/MainCamera.LMB Released` _returnvalue_2)))

(event `Key|RightMouseButton`
  (params (Key :type "Key Structure"))
  (:`Pressed`
    (set `self.rightMousePressed` true)
    ;[1 1 1] Camera Controls
    (bind _returnvalue (`GameplayStatics.GetActorOfClass` "/Game/Blueprints/MainCamera.MainCamera_C"))
    (`/Game/Blueprints/MainCamera.RMB Pressed` _returnvalue))
  (:`Released`
    (set `self.rightMousePressed` false)
    (bind _returnvalue_2 (`GameplayStatics.GetActorOfClass` "/Game/Blueprints/MainCamera.MainCamera_C"))
    (`/Game/Blueprints/MainCamera.RMB Released` _returnvalue_2)))

(event `Drag Actor`
  (params (ScreenSpace :type "Vector2D Structure") (`Actor Reference` :type "Actor Object Reference"))
  (bind (_worldposition _worlddirection) (`GameplayStatics.DeprojectScreenToWorld` self (`SlateBlueprintLibrary.AbsoluteToViewport` ScreenSpace)))
  ;[1 1 1] Drag Actor Custom Event
  (bind _outhit (`KismetSystemLibrary.LineTraceSingle` (`self.K2_GetActorLocation` (`GameplayStatics.GetPlayerCameraManager` 0)) (+ _worldposition (* _worlddirection 5000.0)) "TraceTypeQuery3"))
  (`self.K2_SetActorLocation` `Actor Reference` (`.Location` (`GameplayStatics.BreakHitResult` _outhit)) false false))

(fn `UserConstructionScript`)